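; BP_CurrencyManager registers and exposes a custom token currency for the game.
; On BeginPlay it adds a currency manager under the "CUSTOM_TOKEN" key.
; Its functions look up that manager by key and forward calls to get the amount, add, remove and check whether enough tokens are held, returning the results.
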(event `self.ReceiveBeginPlay`
  (`self.AddManager` "CUSTOM_TOKEN"))

(fn `Add Custom Tokens`
  (params (Amount :type Integer))
  (returns (`New Amount` :type Integer))
  (bind _returnvalue (`self.GetManager` "CUSTOM_TOKEN"))
  (bind _returnvalue_2 (`CurrencyManagerComponent.Add` _returnvalue (`local.Amount`)))
  (return _returnvalue_2))

(fn `Get Custom Tokens`
  (returns (Amount :type Integer))
  (bind _returnvalue (`self.GetManager` "CUSTOM_TOKEN"))
  (return (`CurrencyManagerComponent.GetAmount` _returnvalue)))

(fn `Have Enough Custom Tokens`
  (params (`Required Amount` :type Integer))
  (returns (`Have Enough` :type Boolean))
  (bind _returnvalue (`self.GetManager` "CUSTOM_TOKEN"))
  (return (`CurrencyManagerComponent.HaveEnough` _returnvalue (`local.Required Amount`))))

(fn `Remove Custom Tokens`
  (params (Amount :type Integer))
  (returns (`New Amount` :type Integer))
  (bind _returnvalue (`self.GetManager` "CUSTOM_TOKEN"))
  (bind _returnvalue_2 (`CurrencyManagerComponent.Remove` _returnvalue (`local.Amount`)))
  (return _returnvalue_2))

(fn `UserConstructionScript`)